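; Pig animal AI that roams, eats, rests, flees from perceived stimuli and projectile hits, and dies when health runs out.
; DecideNextAction is the central selector, prioritising fleeing, hunger, then tiredness over random roaming via AIMoveTo.
; Self-calling one-second delay loops drain and refill hunger and energy, re-triggering the selector when either empties.
; Actions play one-off animations directly on the mesh, then StopAnimation restores PigAnimBP; eating first runs a downward ground trace.
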(event OnTargetPerceptionUpdated(AIPerception)
  (params (Actor :type Actor%20Object%20Reference) (Stimulus :type AI%20Stimulus%20Structure))
  ;[1 1 1] Detect Noise
  (if (not (Variables|Default|GetShouldRun?))
    (Variables|Default|SetShouldRun? (.bSuccessfullySensed (Utilities|Struct|BreakAIStimulus Stimulus)))
    (CallFunction|DecideNextAction true)))

(event OnComponentHit(Hitbox)
  (params (HitComponent :type Primitive%20Component%20Object%20Reference) (OtherActor :type Actor%20Object%20Reference) (OtherComp :type Primitive%20Component%20Object%20Reference) (NormalImpulse :type Vector :default "0, 0, 0") (Hit :type Hit%20Result%20Structure%20%28by%20ref%29)))

(event Custom|DecideNextAction
  (params (SkipDelay? :type Boolean))
  ;[1 1 1] Decide Next Action
  (if SkipDelay?
    _
    (else
      (Utilities|FlowControl|Delay (Math|Conversions|ToFloat(Integer) (Math|Random|RandomIntegerinRange 1 5)))))
  (CallFunction|StopAnimation)
  (if (Variables|Default|GetShouldRun?)
    (CallFunction|Runaway)
    (elif (Variables|Default|GetIsHungry?)
      (CallFunction|Eat)
      (elif (Variables|Default|GetIs%20Tired?)
        (CallFunction|Rest)
        (CallFunction|RegainEnergy)
        (else
          (CallFunction|RandomRoam))))))

(event Custom|Regain%20Energy
  ;[1 1 1] Regain Energy
  (if (Variables|Default|GetIs%20Tired?)
    (bind _output_get (Variables|Default|SetEnergy%20 (Math|Integer|Clamp(Integer) (+ (Variables|Default|GetEnergy%20) (Variables|Default|GetEnergy%20Gain)) 0 (Variables|Default|GetMax%20Energy))))
    (if (not (== _output_get (Variables|Default|GetMax%20Energy)))
      (Utilities|FlowControl|Delay 1.0)
      (CallFunction|RegainEnergy))))

(event Custom|Add%20Hunger
  ;[1 1 1] Regen Hunger
  (if (Variables|Default|GetIsHungry?)
    (bind _output_get (Variables|Default|SetHunger (Math|Integer|Clamp(Integer) (+ (Variables|Default|GetHunger) (Variables|Default|GetHungerGain)) 0 (Variables|Default|GetMaxHunger))))
    (if (not (== _output_get (Variables|Default|GetMaxHunger)))
      (Utilities|FlowControl|Delay 1.0)
      (CallFunction|AddHunger))))

(event Custom|Eat
  ;[1 1 1] Eat Anim
  (Utilities|CanEat
    (:Out
      (if true
        (Components|Movement|StopMovementImmediately (Variables|Character|GetCharacterMovement))
        (CallFunction|AddHunger)
        (CallFunction|PlayAnimation "/Game/AnimalVarietyPack/Pig/Animations/ANIM_Pig_SniffleforFood.ANIM_Pig_SniffleforFood" true)
        (Utilities|FlowControl|Delay (Math|Conversions|ToFloat(Integer) (Math|Random|RandomIntegerinRange 5 10)))
        (CallFunction|StopAnimation)
        (Variables|Default|SetIsHungry? false)
        (CallFunction|DrainHunger)
        (CallFunction|DecideNextAction false)
        (else
          (CallFunction|DecideNextAction false)
          (Variables|Default|SetIsHungry? false)
          (Utilities|FlowControl|Delay 5.0)
          (Variables|Default|SetIsHungry? true))))))

(event Custom|Drain%20Hunger
  ;[1 1 1] Drain Hunger
  (if (not (Variables|Default|GetIsHungry?))
    (bind _output_get (Variables|Default|SetHunger (Math|Integer|Clamp(Integer) (- (Variables|Default|GetHunger) (Variables|Default|GetHungerDrain)) 0 (Variables|Default|GetMaxHunger))))
    (if (== _output_get 0)
      (Variables|Default|SetIsHungry? true)
      (CallFunction|DecideNextAction false)
      (else
        (Utilities|FlowControl|Delay 1.0)
        (CallFunction|DrainHunger)))))

(event Custom|Drain%20Energy
  ;[1 1 1] Drain Energy
  (if (not (Variables|Default|GetIs%20Tired?))
    (bind _output_get (Variables|Default|SetEnergy%20 (Math|Integer|Clamp(Integer) (- (Variables|Default|GetEnergy%20) (Variables|Default|GetEnergy%20Drain)) 0 (Variables|Default|GetMax%20Energy))))
    (if (== _output_get 0)
      (Variables|Default|SetIs%20Tired? true)
      (CallFunction|DecideNextAction false)
      (else
        (Utilities|FlowControl|Delay 1.0)
        (CallFunction|DrainEnergy)))))

(event Custom|Runaway
  ;[1 1 1] Run Away
  (CallFunction|StopAnimation)
  (Variables|/Script/Engine.CharacterMovementComponent|SetMaxWalkSpeed (Variables|Character|GetCharacterMovement) 6e+02)
  (AI|AIMoveTo self (.RandomLocation (AI|Navigation|GetRandomReachablePointinRadius (Transformation|GetActorLocation) (Math|Random|RandomFloatinRange 5e+04 1e+05) 0 0)) 0 5.0 false
    (:OnSuccess
      (Variables|Default|SetShouldRun? false)
      (CallFunction|DecideNextAction false))))

(event Custom|Rest
  ;[1 1 1] Sleep Anim
  (Components|Movement|StopMovementImmediately (Variables|Character|GetCharacterMovement))
  (CallFunction|PlayAnimation "/Game/AnimalVarietyPack/Pig/Animations/ANIM_Pig_GoToRest.ANIM_Pig_GoToRest" false)
  (Utilities|FlowControl|Delay 1.4)
  (CallFunction|PlayAnimation "/Game/AnimalVarietyPack/Pig/Animations/ANIM_Pig_Rest.ANIM_Pig_Rest" true)
  (Utilities|FlowControl|Delay (Math|Conversions|ToFloat(Integer) (Math|Random|RandomIntegerinRange 20 30)))
  (CallFunction|PlayAnimation "/Game/AnimalVarietyPack/Pig/Animations/ANIM_Pig_GoBackUp.ANIM_Pig_GoBackUp" false)
  (Utilities|FlowControl|Delay 1.4)
  (CallFunction|StopAnimation)
  (Variables|Default|SetIs%20Tired? false)
  (CallFunction|DecideNextAction false)
  (CallFunction|DrainEnergy))

(event Custom|RandomRoam
  ;[1 1 1] Random Roam
  (Variables|/Script/Engine.CharacterMovementComponent|SetMaxWalkSpeed (Variables|Character|GetCharacterMovement) 1e+02)
  (AI|AIMoveTo self (.RandomLocation (AI|Navigation|GetRandomReachablePointinRadius (Transformation|GetActorLocation) 5e+03 0 0)) 0 5.0 false
    (:then
      (CallFunction|DecideNextAction false))))

(event Custom|GoHome
  ;[1 1 1] Go Home
  (AI|AIMoveTo self (Variables|Default|GetHome) 0 5.0 false
    (:OnSuccess
      (if (Variables|Default|GetIs%20Tired?)
        (CallFunction|Rest)
        (CallFunction|RegainEnergy)
        (else
          (CallFunction|DecideNextAction false))))))

(event Custom|Take%20Damage
  ;[1 1 1] Take Damage
  (if (not (Variables|Default|GetIsDead?))
    (bind _output_get (Variables|Default|SetHealth (Math|Integer|Clamp(Integer) (- (Variables|Default|GetHealth) (Variables|Default|GetDamage)) 0 (Variables|Default|GetMax%20Health))))
    (Audio|PlaySoundatLocation "/Game/AnimalVarietyPack/DeerStagAndDoe/Sounds/Hurt/Hurt.Hurt" (Transformation|GetActorLocation) "0, 0, 0" 1.0 1.0 0.0 0 0 0)
    (if (== _output_get 0)
      (Components|Movement|StopMovementImmediately (Variables|Character|GetCharacterMovement))
      (Variables|Default|SetIsDead? true)
      (Pawn|Components|CharacterMovement|DisableMovement (Variables|Character|GetCharacterMovement))
      (CallFunction|PlayAnimation "/Game/AnimalVarietyPack/Pig/Animations/ANIM_Pig_Death.ANIM_Pig_Death" false)
      (Utilities|FlowControl|Delay 3e+01)
      (Actor|DestroyActor)
      (else
        (Components|Movement|StopMovementImmediately (Variables|Character|GetCharacterMovement))
        (CallFunction|PlayAnimation "/Game/AnimalVarietyPack/Pig/Animations/ANIM_Pig_GetHit.ANIM_Pig_GetHit" false)
        (Variables|Default|SetShouldRun? true)
        (Utilities|FlowControl|Delay 0.7)
        (CallFunction|StopAnimation)
        (if (not (Variables|Default|GetIsDead?))
          (CallFunction|DecideNextAction true))))))

(event EventBeginPlay
  ;[1 1 1] SetUp Blueprint
  (CallFunction|DecideNextAction false)
  (CallFunction|DrainEnergy)
  (CallFunction|DrainHunger))

(event Collision|EventHit
  (params (MyComp :type Primitive%20Component%20Object%20Reference) (Other :type Actor%20Object%20Reference) (OtherComp :type Primitive%20Component%20Object%20Reference) (bSelfMoved :type Boolean) (HitLocation :type Vector :default "0, 0, 0") (HitNormal :type Vector :default "0, 0, 0") (NormalImpulse :type Vector :default "0, 0, 0") (Hit :type Hit%20Result%20Structure%20%28by%20ref%29))
  ;[1 1 1] Projectile Hit
  (bind _asprojectile_bp (Utilities|Casting|CastToProjectileBP Other))
  (Variables|Default|SetDamage 10)
  (CallFunction|TakeDamage)
  (Actor|DestroyActor _asprojectile_bp))

(fn ConstructionScript)

(fn PlayAnimation
  (params (Animation :type Animation%20Asset%20Object%20Reference) (Should%20loop? :type Boolean))
  (Components|Animation|PlayAnimation (Variables|Character|GetMesh) Animation Should%20loop?))

(fn StopAnimation
  (bind _mesh (Variables|Character|GetMesh))
  (Components|Animation|SetAnimationMode _mesh "AnimationBlueprint")
  (Class|SkeletalMeshComponent|SetAnimClass _mesh "/Game/AnimalVarietyPack/Pig/PigAnimBP.PigAnimBP_C"))