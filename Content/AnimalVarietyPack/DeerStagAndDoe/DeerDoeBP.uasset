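; Deer doe wildlife AI that roams, grazes, rests at its Home and flees when it senses a stimulus or is hit.
; DecideNextAction prioritises fleeing, eating, resting, then roaming via AIMoveTo, driven by hunger and energy timers built from self-calling delayed events.
; Grazing requires a downward-trace surface-type check, and actions play one-off mesh animations before restoring the Animation Blueprint.
; ProjectileBP hits deal damage, triggering flight or death with delayed destruction.
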(event OnTargetPerceptionUpdated(AIPerception)
  (params (Actor :type Actor%20Object%20Reference) (Stimulus :type AI%20Stimulus%20Structure))
  ;[1 1 1] Detect Noise
  (if (not (Variables|Default|GetShouldRun?))
    (Variables|Default|SetShouldRun? (.bSuccessfullySensed (Utilities|Struct|BreakAIStimulus Stimulus)))
    (CallFunction|DecideNextAction true)))

(event Custom|DecideNextAction
  (params (SkipDelay? :type Boolean))
  ;[1 1 1] Decide Next Action
  (if SkipDelay?
    _
    (else
      (Utilities|FlowControl|Delay (Math|Conversions|ToFloat(Integer) (Math|Random|RandomIntegerinRange 1 5)))))
  (CallFunction|StopAnimation)
  (if (Variables|Default|GetShouldRun?)
    (CallFunction|Runaway)
    (elif (Variables|Default|GetIsHungry?)
      (CallFunction|Eat)
      (elif (Variables|Default|GetIs%20Tired?)
        (CallFunction|GoHome)
        (else
          (CallFunction|RandomRoam))))))

(event Custom|RandomRoam
  ;[1 1 1] Random Roam
  (Variables|/Script/Engine.CharacterMovementComponent|SetMaxWalkSpeed (Variables|Character|GetCharacterMovement) 1.5e+02)
  (AI|AIMoveTo self (.RandomLocation (AI|Navigation|GetRandomReachablePointinRadius (Transformation|GetActorLocation) 1.5e+03 0 0)) 0 5.0 false
    (:OnSuccess
      (CallFunction|DecideNextAction false))))

(event Custom|Regen
  ;[1 1 1] RegenHealth
  (if (and (< (Variables|Damage|GetHealth) (Variables|Damage|GetMax%20Health)) (not (Variables|Default|GetShouldRun?)))
    (bind _output_get (Variables|Damage|SetHealth (Math|Integer|Clamp(Integer) (+ (Variables|Damage|GetHealth) (Variables|Damage|GetHealthGain)) 0 (Variables|Damage|GetMax%20Health))))
    (if (not (== _output_get (Variables|Damage|GetMax%20Health)))
      (Utilities|FlowControl|Delay 1.0)
      (CallFunction|Regen))))

(event Custom|Add%20Hunger
  ;[1 1 1] Regen Hunger
  (if (Variables|Default|GetIsHungry?)
    (bind _output_get (Variables|Hunger|SetHunger (Math|Integer|Clamp(Integer) (+ (Variables|Hunger|GetHunger) (Variables|Hunger|GetHungerGain)) 0 (Variables|Hunger|GetMaxHunger))))
    (if (not (== _output_get (Variables|Hunger|GetMaxHunger)))
      (Utilities|FlowControl|Delay 1.0)
      (CallFunction|AddHunger))))

(event Custom|Eat
  ;[1 1 1] Eat Anim
  (bind _caneat_ (Utilities|CanEat)
    (:Out
      (if _caneat_
        (Components|Movement|StopMovementImmediately (Variables|Character|GetCharacterMovement))
        (CallFunction|AddHunger)
        (CallFunction|PlayAnimation "/Game/AnimalVarietyPack/DeerStagAndDoe/Animations/ANIM_DeerDoe_GrazeOnce.ANIM_DeerDoe_GrazeOnce" false)
        (Utilities|FlowControl|Delay 1.0)
        (CallFunction|PlayAnimation "/Game/AnimalVarietyPack/DeerStagAndDoe/Animations/ANIM_DeerDoe_IdleGraze.ANIM_DeerDoe_IdleGraze" true)
        (Utilities|FlowControl|Delay (Math|Conversions|ToFloat(Integer) (Math|Random|RandomIntegerinRange 3 10)))
        (CallFunction|PlayAnimation "/Game/AnimalVarietyPack/DeerStagAndDoe/Animations/ANIM_DeerDoe_GrazeEnd.ANIM_DeerDoe_GrazeEnd" false)
        (Utilities|FlowControl|Delay 1.0)
        (CallFunction|StopAnimation)
        (Variables|Default|SetIsHungry? false)
        (CallFunction|DrainHunger)
        (CallFunction|DecideNextAction false)
        (else
          (CallFunction|DecideNextAction false)
          (Variables|Default|SetIsHungry? false)
          (Utilities|FlowControl|Delay 5.0)
          (Variables|Default|SetIsHungry? true))))))

(event Custom|Drain%20Hunger
  ;[1 1 1] Drain Hunger
  (if (not (Variables|Default|GetIsHungry?))
    (bind _output_get (Variables|Hunger|SetHunger (Math|Integer|Clamp(Integer) (- (Variables|Hunger|GetHunger) (Variables|Hunger|GetHungerDrain)) 0 (Variables|Hunger|GetMaxHunger))))
    (if (== _output_get 0)
      (Variables|Default|SetIsHungry? true)
      (CallFunction|DecideNextAction false)
      (else
        (Utilities|FlowControl|Delay 1.0)
        (CallFunction|DrainHunger)))))

(event Custom|Runaway
  ;[1 1 1] Run Away
  (CallFunction|StopAnimation)
  (Variables|/Script/Engine.CharacterMovementComponent|SetMaxWalkSpeed (Variables|Character|GetCharacterMovement) 1e+03)
  (AI|AIMoveTo self (.RandomLocation (AI|Navigation|GetRandomReachablePointinRadius (Transformation|GetActorLocation) (Math|Random|RandomFloatinRange 5e+04 1e+05) 0 0)) 0 5.0 false
    (:OnSuccess
      (Variables|Default|SetShouldRun? false)
      (CallFunction|DecideNextAction false))))

(event Custom|Rest
  ;[1 1 1] Sleep Anim
  (Components|Movement|StopMovementImmediately (Variables|Character|GetCharacterMovement))
  (CallFunction|PlayAnimation "/Game/AnimalVarietyPack/DeerStagAndDoe/Animations/ANIM_DeerDoe_GoToRest.ANIM_DeerDoe_GoToRest" false)
  (Utilities|FlowControl|Delay 1.4)
  (CallFunction|PlayAnimation "/Game/AnimalVarietyPack/DeerStagAndDoe/Animations/ANIM_DeerDoe_IdleRest.ANIM_DeerDoe_IdleRest" true)
  (Utilities|FlowControl|Delay (Math|Conversions|ToFloat(Integer) (Math|Random|RandomIntegerinRange 20 30)))
  (CallFunction|PlayAnimation "/Game/AnimalVarietyPack/DeerStagAndDoe/Animations/ANIM_DeerDoe_RestToGoBackUp.ANIM_DeerDoe_RestToGoBackUp" false)
  (Utilities|FlowControl|Delay 1.4)
  (CallFunction|StopAnimation)
  (Variables|Default|SetIs%20Tired? false)
  (CallFunction|DecideNextAction false)
  (CallFunction|DrainEnergy))

(event Custom|Drain%20Energy
  ;[1 1 1] Drain Energy
  (if (not (Variables|Default|GetIs%20Tired?))
    (bind _output_get (Variables|Energy|SetEnergy%20 (Math|Integer|Clamp(Integer) (- (Variables|Energy|GetEnergy%20) (Variables|Energy|GetEnergy%20Drain)) 0 (Variables|Energy|GetMax%20Energy))))
    (if (== _output_get 0)
      (Variables|Default|SetIs%20Tired? true)
      (CallFunction|DecideNextAction false)
      (else
        (Utilities|FlowControl|Delay 1.0)
        (CallFunction|DrainEnergy)))))

(event Custom|Regain%20Energy
  ;[1 1 1] Regain Energy
  (if (Variables|Default|GetIs%20Tired?)
    (bind _output_get (Variables|Energy|SetEnergy%20 (Math|Integer|Clamp(Integer) (+ (Variables|Energy|GetEnergy%20) (Variables|Energy|GetEnergy%20Gain)) 0 (Variables|Energy|GetMax%20Energy))))
    (if (not (== _output_get (Variables|Energy|GetMax%20Energy)))
      (Utilities|FlowControl|Delay 1.0)
      (CallFunction|RegainEnergy))))

(event Custom|GoHome
  ;[1 1 1] Go Home
  (AI|AIMoveTo self (Variables|Default|GetHome) 0 5.0 false
    (:OnSuccess
      (if (Variables|Default|GetIs%20Tired?)
        (CallFunction|Rest)
        (CallFunction|RegainEnergy)
        (else
          (CallFunction|DecideNextAction false))))))

(event Custom|Take%20Damage
  ;[1 1 1] Take Damage
  (if (not (Variables|Damage|GetIsDead?))
    (bind _output_get (Variables|Damage|SetHealth (Math|Integer|Clamp(Integer) (- (Variables|Damage|GetHealth) (Variables|Damage|GetDamage)) 0 (Variables|Damage|GetMax%20Health))))
    (Audio|PlaySoundatLocation "/Game/AnimalVarietyPack/DeerStagAndDoe/Sounds/Hurt/Hurt.Hurt" (Transformation|GetActorLocation) "0, 0, 0" 1.0 1.0 0.0 0 0 0)
    (if (== _output_get 0)
      (Components|Movement|StopMovementImmediately (Variables|Character|GetCharacterMovement))
      (Variables|Damage|SetIsDead? true)
      (Pawn|Components|CharacterMovement|DisableMovement (Variables|Character|GetCharacterMovement))
      (CallFunction|PlayAnimation "/Game/AnimalVarietyPack/DeerStagAndDoe/Animations/ANIM_DeerDoe_Death.ANIM_DeerDoe_Death" false)
      (Utilities|FlowControl|Delay 3e+01)
      (Actor|DestroyActor)
      (else
        (Components|Movement|StopMovementImmediately (Variables|Character|GetCharacterMovement))
        (CallFunction|PlayAnimation "/Game/AnimalVarietyPack/DeerStagAndDoe/Animations/ANIM_DeerDoe_GetHit.ANIM_DeerDoe_GetHit" false)
        (Variables|Default|SetShouldRun? true)
        (Utilities|FlowControl|Delay 0.7)
        (CallFunction|StopAnimation)
        (if (not (Variables|Damage|GetIsDead?))
          (CallFunction|DecideNextAction true))))))

(event EventBeginPlay
  ;[1 1 1] SetUp Blueprint
  (CallFunction|DecideNextAction false)
  (CallFunction|DrainEnergy)
  (CallFunction|DrainHunger))

(event Collision|EventHit
  (params (MyComp :type Primitive%20Component%20Object%20Reference) (Other :type Actor%20Object%20Reference) (OtherComp :type Primitive%20Component%20Object%20Reference) (bSelfMoved :type Boolean) (HitLocation :type Vector :default "0, 0, 0") (HitNormal :type Vector :default "0, 0, 0") (NormalImpulse :type Vector :default "0, 0, 0") (Hit :type Hit%20Result%20Structure%20%28by%20ref%29))
  ;[1 1 1] Projectile Hit
  (bind _asprojectile_bp (Utilities|Casting|CastToProjectileBP Other))
  (Variables|Damage|SetDamage 10)
  (CallFunction|TakeDamage)
  (Actor|DestroyActor _asprojectile_bp))

(fn ConstructionScript)

(fn PlayAnimation
  (params (Animation :type Animation%20Asset%20Object%20Reference) (Should%20loop? :type Boolean))
  (Components|Animation|PlayAnimation (Variables|Character|GetMesh) Animation Should%20loop?))

(fn StopAnimation
  (bind _mesh (Variables|Character|GetMesh))
  (Components|Animation|SetAnimationMode _mesh "AnimationBlueprint")
  (Class|SkeletalMeshComponent|SetAnimClass _mesh "/Game/AnimalVarietyPack/DeerStagAndDoe/DeerDoeAnimBP.DeerDoeAnimBP_C"))

(fn Shapeshifting
  (return true))